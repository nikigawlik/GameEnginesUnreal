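; Player cube for an endless spline-following racer that steers around the track axis, counts laps and dies on obstacles.
; BeginPlay finds the starting spline distance; Tick moves the grandparent actor along the looping spline at ever-increasing speed while damped horizontal input rotates the parent actor.
; Overlaps matched by actor name prefix update the HUD lap counter or show the end screen, after which any key reloads the level.
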(event EventBeginPlay
  (bind _splineblueprint (Variables|CubeControl|GetsplineBlueprint))
  (bind _spline (Variables|/Game/Blueprints/SplineBlueprint.SplineBlueprint_C|GetSpline _splineblueprint))
  ;[1 1 1] Calculate start position based on closest point on spline
  (while (or (> (Math|Vector|VectorLength (- (Spline|GetLocationatDistanceAlongSpline _spline (Variables|CubeControl|GetpositionOnSpline) "World") (Spline|FindLocationClosesttoWorldLocation _spline (Transformation|GetActorLocation) "World"))) 1e+02) (> (Variables|CubeControl|GetpositionOnSpline) (Spline|GetSplineLength _spline)))
    (Variables|CubeControl|SetpositionOnSpline (+ (Variables|CubeControl|GetpositionOnSpline) 5e+01))))

(event EventTick
  (params (DeltaSeconds :type Float%20%28single-precision%29))
  (bind _returnvalue (Actor|GetAttachParentActor))
  (bind _splineblueprint (Variables|CubeControl|GetsplineBlueprint))
  (bind _spline (Variables|/Game/Blueprints/SplineBlueprint.SplineBlueprint_C|GetSpline _splineblueprint))
  (if (not (Variables|Default|Getdead))
    (Utilities|FlowControl|Sequence
      (:then_0
        ;[1 1 1] Movement System
        (bind _output_get (Variables|CubeControl|Setspeed (/ (+ (Variables|CubeControl|Getspeed) (* DeltaSeconds (Variables|CubeControl|Getacceleration) (Input|AxisValues|GetHorizontal))) (+ (* (Variables|CubeControl|Getdamping) DeltaSeconds) 1.0))))
        (Transformation|AddActorLocalRotation _returnvalue (* "1.000000, 0, 0" (* _output_get DeltaSeconds)) false false))
      (:then_1
        (bind _output_get_2 (Variables|CubeControl|SetpositionOnSpline (Math|Float|%(Float) (+ (Variables|CubeControl|GetpositionOnSpline) (* DeltaSeconds (Variables|CubeControl|GetforwardSpeed))) (Spline|GetSplineLength _spline))))
        (Transformation|SetActorLocationAndRotation (Actor|GetAttachParentActor _returnvalue) (Spline|GetLocationatDistanceAlongSpline _spline _output_get_2 "World") (Class|KismetMathLibrary|MakeRotfromYZ (Spline|GetTangentatDistanceAlongSpline _spline _output_get_2 "Local") (Class|SplineComponent|GetRightVectoratDistanceAlongSpline _spline _output_get_2 "Local"))))
      (:then_2
        (Variables|CubeControl|SetforwardSpeed (+ (Variables|CubeControl|GetforwardSpeed) (* DeltaSeconds (Variables|CubeControl|GetspeedIncreaseOverTime))))))))

(event Collision|EventActorBeginOverlap
  (params (OtherActor :type Actor%20Object%20Reference))
  (bind _returnvalue (Utilities|GetObjectName OtherActor))
  ;[1 1 1] Collision
  (Utilities|FlowControl|Sequence
    (:then_0
      (Development|PrintString _returnvalue))
    (:then_1
      (if (Utilities|String|StartsWith _returnvalue "finishLineTrigger")
        ;[1 1 1] Update Lap Counter
        (bind _ascustom_hud (Utilities|Casting|CastToCustomHUD (HUD|GetHUD (Game|GetPlayerController 0))))
        (Default|UpdateUI(NewLap) (Variables|/Game/Blueprints/CustomHUD.CustomHUD_C|GethudWidget _ascustom_hud))
        (Development|PrintString "Lap!")))
    (:then_2
      (if (Utilities|String|StartsWith _returnvalue "obstacle")
        ;[1 1 1] Game Over
        (Variables|Default|Setdead true)
        (bind _ascustom_hud_2 (Utilities|Casting|CastToCustomHUD (HUD|GetHUD (Game|GetPlayerController 0))))
        (Default|SetEndScreen _ascustom_hud_2)
        (Development|PrintString "Dead")))))

(event Input|KeyboardEvents|AnyKey
  (params (Key :type Key%20Structure))
  ;[1 1 1] Restart Game
  (:Pressed
    (if (Variables|Default|Getdead)
      (bind _returnvalue (Game|GetCurrentLevelName true))
      (Game|OpenLevel(byName) (Utilities|String|StringToName _returnvalue)))))

(fn ConstructionScript)