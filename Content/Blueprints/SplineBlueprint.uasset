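; Spline Blueprint actor that builds a closed loop of spline mesh segments along its Spline component.
; The construction script adds one spline mesh component per spline point and attaches it to the default scene root.
; Each segment takes its local position and tangent from that point and the next, with a modulo wrap joining the last point back to the first.
; The event graph has no active logic.
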(event EventBeginPlay)

(event Collision|EventActorBeginOverlap
  (params (OtherActor :type Actor%20Object%20Reference)))

(event EventTick
  (params (DeltaSeconds :type Float%20%28single-precision%29)))

(fn ConstructionScript
  (bind _spline (Variables|Default|GetSpline))
  (bind _returnvalue (Spline|GetNumberOfSplinePoints _spline))
  (for _index (range 0 (- _returnvalue 1))
    (bind _returnvalue_2 (AddComponent|AddSplineMeshComponent true))
    (Transformation|AttachComponentToComponent _returnvalue_2 (Variables|Default|GetDefaultSceneRoot) "SplineMEshes" "KeepRelative" "KeepRelative" "KeepRelative" true)
    (SplineMesh|SetStartandEnd _returnvalue_2 (.Location (Spline|GetLocationandTangentatSplinePoint _spline _index "Local")) (.Tangent (Spline|GetLocationandTangentatSplinePoint _spline _index "Local")) (.Location (Spline|GetLocationandTangentatSplinePoint _spline (Math|Integer|%(Integer) (+ _index 1) _returnvalue) "Local")) (.Tangent (Spline|GetLocationandTangentatSplinePoint _spline (Math|Integer|%(Integer) (+ _index 1) _returnvalue) "Local")) true :!class /Script/Engine.SplineMeshComponent)))